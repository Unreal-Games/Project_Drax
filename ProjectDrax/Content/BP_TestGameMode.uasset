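; Test game mode that spawns AI bots through EQS and handles kill scoring.
; SpawnNewBot runs a single-result EQS query, whose finish handler draws debug spheres and spawns BP_BotAI at result locations.
; The loop is also reached through a second sequence branch that bypasses the success check.
; A kill delegate bound at BeginPlay calls AddScore with zero for non-player victims and prints the killer's score.
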(event `self.SpawnNewBot`
  (bind _returnvalue (`EnvQueryManager.RunEQSQuery` "/Game/EQS/EQS_BotSpawn.EQS_BotSpawn" self "SingleResult"))
  (add `EnvQueryInstanceBlueprintWrapper.OnQueryFinishedEvent` _returnvalue (delegate `OnQueryFinishedEvent`)))

(event `OnQueryFinishedEvent`
  (params (QueryInstance :type "EnvQueryInstanceBlueprintWrapper Object Reference") (QueryStatus :type "EEnvQueryStatus Enum" :default "Processing"))
  (`|ExecutionSequence`
    (:`then_0`
      (switch `EEnvQueryStatus` QueryStatus
        (:`Success`
          _)))
    (:`then_1`
      (bind _resultlocations (`EnvQueryInstanceBlueprintWrapper.GetQueryResultsAsLocations` QueryInstance))))
  (for _array_element _resultlocations
    (`KismetSystemLibrary.DrawDebugSphere` _array_element 50.0 12 (struct :`R` 1.0 :`G` 0.97434 :`B` 0.358465 :`A` 1.0) 2.0 2.0)
    (`|SpawnActorFromClass` "/Game/AI_Bot/BP_BotAI.BP_BotAI_C" (`KismetMathLibrary.MakeTransform` _array_element) "AdjustIfPossibleButDontSpawnIfColliding" "OverrideRootScale" null null)))

(event `self.ReceiveBeginPlay`
  (add `self.OnActorKilled` (delegate `OnActorKilled_Event_0`)))

(event `OnActorKilled_Event_0` :!signature `self.OnActorKilled`
  (params (VictimActor :type "Actor Object Reference") (KillerActor :type "Actor Object Reference") (KillerController :type "Controller Object Reference"))
  (bind _playerstate (`Pawn.PlayerState` (`Controller.K2_GetPawn` KillerController)))
  (bind _aspawn (cast `Pawn` VictimActor))
  (if (not (`Pawn.IsPlayerControlled` _aspawn))
    (bind _assplayer_state (cast `SPlayerState` _playerstate))
    (`SPlayerState.AddScore` _assplayer_state 0.0)
    (`KismetSystemLibrary.PrintString` (`KismetStringLibrary.Conv_DoubleToString` (`PlayerState.Score` _playerstate)))))

(fn `UserConstructionScript`)