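; BP_RecordingActor is an inventory preview double of the player character that displays its mesh and weapons and can be rotated by dragging.
; BeginPlay, every Tick and the J key copy BP_Character's mesh and first two WeaponInventory meshes, re-attaching the weapons to sockets.
; The secondary weapon updates only when a primary exists.
; ClickedStart, MouseMove and ClickedEnd turn horizontal mouse movement into yaw on the skeletal mesh.
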(event `Key|J`
  (params (Key :type "Key Structure"))
  (bind _secondaryweapon (`self.SecondaryWeapon`))
  (:`Pressed`
    (bind _asbp_character (cast `/Game/BP_Character` (`GameplayStatics.GetPlayerCharacter` 0) :!label _label))
    (`SkinnedMeshComponent.SetSkinnedAssetAndUpdate` (`self.SkeletalMesh`) (`SkinnedMeshComponent.SkeletalMesh` (`Character.Mesh` _asbp_character)) false)
    (bind _weaponinventory (`DCharacter.WeaponInventory` _asbp_character))
    (bind _output (`|GetArrayItem` _weaponinventory))
    (`/Engine/EditorBlueprintResources/StandardMacros.IsValid` _output
      (:`Is Valid`
        (`SkinnedMeshComponent.SetSkinnedAssetAndUpdate` (`self.PrimaryWeapon`) (`SkinnedMeshComponent.SkeletalMesh` (`DWeapon.MeshComp` _output)) false)
        (`SceneComponent.K2_AttachToComponent` (`self.PrimaryWeapon`) (`self.SkeletalMesh`) "GunSocket" "SnapToTarget" "SnapToTarget" "SnapToTarget" true)
        (bind _output_2 (`|GetArrayItem` _weaponinventory 1))
        (`/Engine/EditorBlueprintResources/StandardMacros.IsValid` _output_2
          (:`Is Valid`
            (`SkinnedMeshComponent.SetSkinnedAssetAndUpdate` _secondaryweapon (`SkinnedMeshComponent.SkeletalMesh` (`DWeapon.MeshComp` _output_2)) false)
            (`SceneComponent.K2_AttachToComponent` _secondaryweapon (`self.SkeletalMesh`) "Weapon1" "SnapToTarget" "SnapToTarget" "KeepRelative" false)))))))

(event `self.ReceiveTick`
  (params (DeltaSeconds :type "Float (single-precision)"))
  (goto _label))

(event `self.ReceiveBeginPlay`
  (goto _label))

(event `ClickedStart`
  (params (`Mouse Location` :type "Vector2D Structure"))
  (set `self.StartLocation` `Mouse Location`)
  (set `self.bCanRotate` true))

(event `ClickedEnd`
  (set `self.bCanRotate` false))

(event `Mouse Move`
  (params (`Mouse Location` :type "Vector2D Structure"))
  (bind _returnvalue_x (`KismetMathLibrary.BreakVector2D` (- `Mouse Location` (`self.StartLocation`))))
  (if (`self.bCanRotate`)
    (`SceneComponent.K2_AddWorldRotation` (`self.SkeletalMesh`) (`KismetMathLibrary.MakeRotator` 0.0 0.0 (* -1 _returnvalue_x)) false false)
    (set `self.StartLocation` `Mouse Location`)))

(fn `UserConstructionScript`)