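; Weapon Blueprint that shows and hides a scope overlay for aiming down sights (ADS).
; ShowADSOverlay creates a new HUD_Scope widget for player controller 0 on each call, stores it as ADS and adds it to the viewport.
; HideADSOverlay removes that stored widget from its parent.
; BeginPlay is empty, and the logic that would create a WBP_Weapon widget is disconnected, so it never runs.
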(event `self.ReceiveBeginPlay`)

(event `self.ShowADSOverlay`
  (bind _returnvalue (`GameplayStatics.GetPlayerController` 0))
  (`/Engine/EditorBlueprintResources/StandardMacros.IsValid` _returnvalue
    (:`Is Valid`
      (bind _returnvalue_2 (`|CreateWidget` "/Game/Weapon/HUD_Scope.HUD_Scope_C" _returnvalue))
      (bind _output_get (set `self.ADS` _returnvalue_2))
      (`UserWidget.AddToViewport` _output_get 0))))

(event `self.HideADSOverlay`
  (`Widget.RemoveFromParent` (`self.ADS`)))

(fn `UserConstructionScript`)