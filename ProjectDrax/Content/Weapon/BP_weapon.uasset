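; BP_weapon is a weapon Blueprint that manages the weapon UI and an aim-down-sights scope overlay.
; On BeginPlay it creates a WBP_Weapon widget and adds it to the viewport.
; ShowADSOverlay creates a new HUD_Scope for the first player controller on each call, if that controller is valid, and stores it in ADS.
; HideADSOverlay removes that stored widget from its parent without a validity check.
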(event `self.ReceiveBeginPlay`
  (bind _returnvalue (`|CreateWidget` "/Game/UI/WBP_Weapon.WBP_Weapon_C"))
  (`UserWidget.AddToViewport` _returnvalue 0))

(event `self.ShowADSOverlay`
  (bind _returnvalue (`GameplayStatics.GetPlayerController` 0))
  (`/Engine/EditorBlueprintResources/StandardMacros.IsValid` _returnvalue
    (:`Is Valid`
      (bind _returnvalue_2 (`|CreateWidget` "/Game/Weapon/HUD_Scope.HUD_Scope_C" _returnvalue))
      (bind _output_get (set `self.ADS` _returnvalue_2))
      (`UserWidget.AddToViewport` _output_get 0))))

(event `self.HideADSOverlay`
  (`Widget.RemoveFromParent` (`self.ADS`)))

(fn `UserConstructionScript`)