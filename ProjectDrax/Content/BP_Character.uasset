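; Player character Blueprint that sets up the local player's HUD and handles inventory screen toggling.
; On BeginPlay, if locally controlled, it adds crosshair, health and weapon widgets (a second weapon widget if CurrentWeapon is valid), caches the Inventory component and spawns a BP_RecordingActor at a random far-off location.
; ShowInventory flip-flops between scanning nearby items to build the lazily created, reused inventory widget and hiding it, switching input mode and cursor.
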(event `self.ReceiveBeginPlay`
  (bind _returnvalue (`GameplayStatics.GetPlayerPawn` 0))
  (bind _returnvalue_2 (* (`KismetMathLibrary.RandomFloatInRange` 1.0 2.0) 1000000.0))
  (if (`self.IsLocallyControlled`)
    (`|ExecutionSequence`
      (:`then_0`
        (bind _returnvalue_3 (`|CreateWidget` "/Game/UI/WBP_Crosshair.WBP_Crosshair_C"))
        (`UserWidget.AddToViewport` _returnvalue_3 0))
      (:`then_1`
        (bind _returnvalue_4 (`|CreateWidget` "/Game/UI/WBP_HealthIndicator.WBP_HealthIndicator_C"))
        (`UserWidget.AddToViewport` _returnvalue_4 0))
      (:`then_2`
        (bind _returnvalue_5 (`|CreateWidget` "/Game/UI/WBP_Weapon.WBP_Weapon_C"))
        (`UserWidget.AddToViewport` _returnvalue_5 0))
      (:`then_3`
        (bind _asdcharacter (cast `DCharacter` _returnvalue))
        (`/Engine/EditorBlueprintResources/StandardMacros.IsValid` (`DCharacter.CurrentWeapon` _asdcharacter)
          (:`Is Valid`
            (bind _returnvalue_6 (`|CreateWidget` "/Game/UI/WBP_Weapon.WBP_Weapon_C"))
            (`UserWidget.AddToViewport` _returnvalue_6 0))))
      (:`then_4`
        (set `self.Inventory` (`self.GetComponentByClass` _returnvalue "/Script/ProjectDrax.Inventory")))
      (:`then_5`
        (bind _returnvalue_7 (`|SpawnActorFromClass` "/Game/Inventory/BP_RecordingActor.BP_RecordingActor_C" (`KismetMathLibrary.MakeTransform` (`KismetMathLibrary.MakeVector` _returnvalue_2 _returnvalue_2 _returnvalue_2)) "Undefined" "OverrideRootScale" null null))
        (set `self.RecordingRef` _returnvalue_7)))))

(event `self.ShowInventory`
  (bind _wbp_inventoryref (`self.WBP_InventoryRef`))
  (`/Engine/EditorBlueprintResources/StandardMacros.FlipFlop`
    (:`A`
      (`self.Construct Inventory`))
    (:`B`
      (`self.Game UI`)
      (`/Engine/EditorBlueprintResources/StandardMacros.IsValid` _wbp_inventoryref
        (:`Is Valid`
          (`Widget.SetVisibility` _wbp_inventoryref "Hidden"))))))

(event `Construct Inventory`
  (bind _inventory (`self.Inventory`))
  (bind _wbp_inventoryref (`self.WBP_InventoryRef`))
  (`/Engine/EditorBlueprintResources/StandardMacros.IsValid` _inventory
    (:`Is Valid`
      (`Inventory.FindNearByItems` _inventory)
      (`self.Inventory UI`)
      (`/Engine/EditorBlueprintResources/StandardMacros.IsValid` _wbp_inventoryref
        (:`Is Valid`
          (`Widget.SetVisibility` _wbp_inventoryref "Visible")
          (`/Game/Inventory/InventoryUI/WBP_InventoryMain.BuildInventory` _wbp_inventoryref))
        (:`Is Not Valid`
          (bind _returnvalue (`|CreateWidget` "/Game/Inventory/InventoryUI/WBP_InventoryMain.WBP_InventoryMain_C"))
          (bind _output_get (set `self.WBP_InventoryRef` _returnvalue))
          (`UserWidget.AddToViewport` _output_get 0)
          (`/Game/Inventory/InventoryUI/WBP_InventoryMain.BuildInventory` _output_get))))))

(event `Inventory UI`
  (bind _returnvalue (`GameplayStatics.GetPlayerController` 0))
  (set `PlayerController.bShowMouseCursor` true _returnvalue)
  (`WidgetBlueprintLibrary.SetInputMode_GameAndUIEx` _returnvalue null "DoNotLock" false))

(event `Game UI`
  (bind _returnvalue (`GameplayStatics.GetPlayerController` 0))
  (set `PlayerController.bShowMouseCursor` false _returnvalue)
  (`WidgetBlueprintLibrary.SetInputMode_GameOnly` _returnvalue))

(fn `UserConstructionScript`)